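; An interactable door that swings open and closed, and can be locked so that the player must spend a key on first use.
; BeginPlay caches the player's ThirdPersonCharacter, whose KeyCount InteractDoor checks and decrements to clear NeedKey, playing a no-key sound and message otherwise.
; Each successful interaction toggles InteractState, plays the matching sound and runs a Timeline forward or in reverse to lerp the actor's relative rotation.
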(event EventInteractDoor
  (if (Variables|Default|GetNeedKey?)
    (if (> (Variables|/Game/ThirdPersonBP/Blueprints/ThirdPersonCharacter.ThirdPersonCharacter_C|GetKeyCount (stale EventBeginPlay _asthird_person_character)) 0)
      (bind _result (Math|Integer|DecrementInt (Variables|/Game/ThirdPersonBP/Blueprints/ThirdPersonCharacter.ThirdPersonCharacter_C|GetKeyCount (stale EventBeginPlay _asthird_person_character)))
        (:%20%20
          (Variables|/Game/ThirdPersonBP/Blueprints/ThirdPersonCharacter.ThirdPersonCharacter_C|SetKeyCount (stale EventBeginPlay _asthird_person_character) _result)
          (Variables|Default|SetNeedKey? false)
          (Development|PrintString "Open Door" :!label _label)
          (if (Variables|Default|GetInteract%20State)
            (Variables|Default|SetInteract%20State false)
            (Audio|PlaySound2D "/Game/Sounds/Door/door_close.door_close" 1.0 1.0 0.0 0 0)
            (bind _track (Timeline|Timeline Reverse)
              (:Update
                (Transformation|SetActorRelativeRotation (Math|Rotator|Lerp(Rotator) (Variables|Default|GetStartRotation) (Variables|Default|GetEndRotation) _track))))
            (else
              (Variables|Default|SetInteract%20State true)
              (Audio|PlaySound2D "/Game/Sounds/Door/door_open.door_open" 1.0 1.0 0.0 0 0)
              (Timeline|Timeline Play)))))
      (else
        (Audio|PlaySound2D "/Game/Sounds/Door/door_no_key.door_no_key" 1.0 1.0 0.0 0 0)
        (Development|PrintString "Tu n'as pas de clé")))
    (else
      (goto _label))))

(event EventBeginPlay
  (bind _asthird_person_character (Utilities|Casting|CastToThirdPersonCharacter (Game|GetPlayerCharacter 0))))

(fn ConstructionScript)